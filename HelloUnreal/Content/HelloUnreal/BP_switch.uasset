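; Overlap switch that starts and stops referenced actors through its Cube component.
; Begin Overlap sets IsPlay on MoveActor, MoveRect and MoveStair and calls DoSpawn on Spawner, while End Overlap only clears the IsPlay flags.
; Each reference is validity-checked in its own Sequence branch, so a missing one prints an error without blocking the others.
; Both events print overlap details for debugging, and two unconnected older stop chains remain in the graph.
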(event OnComponentBeginOverlap(Cube)
  (params (OverlappedComponent :type Primitive%20Component%20Object%20Reference) (OtherActor :type Actor%20Object%20Reference) (OtherComp :type Primitive%20Component%20Object%20Reference) (OtherBodyIndex :type Integer) (bFromSweep :type Boolean) (SweepResult :type Hit%20Result%20Structure%20%28by%20ref%29))
  (Development|PrintString (Utilities|String|Append "Begin Overlap" "Overlapped Component :" (Utilities|GetDisplayName OverlappedComponent) ". Other Actor :" (Utilities|GetDisplayName OtherActor) ". Other Comp :" (Utilities|GetDisplayName OtherComp)) true true "(R=0.000000,G=0.660000,B=1.000000,A=1.000000)" 6e+01)
  (Utilities|FlowControl|Sequence
    (:then_0
      (Utilities|IsValid (Variables|Default|GetMoveActor)
        (:Is%20Valid
          (Variables|/Game/HelloUnreal/BP_MoveActor.BP_MoveActor_C|SetIsPlay (Variables|Default|GetMoveActor) true))
        (:Is%20Not%20Valid
          (Development|PrintString "MoveActor is Nullptr!!" true true "(R=0.520001,G=0.000000,B=0.000000,A=1.000000)"))))
    (:then_1
      (Utilities|IsValid (Variables|Default|GetMoveRect)
        (:Is%20Valid
          (Variables|/Game/HelloUnreal/BP_MoveRect.BP_MoveRect_C|SetIsPlay (Variables|Default|GetMoveRect) true))
        (:Is%20Not%20Valid
          (Development|PrintString "MoveRect is Nullptr!!" true true "(R=0.520001,G=0.000000,B=0.000000,A=1.000000)"))))
    (:then_2
      (Utilities|IsValid (Variables|Default|GetMoveStair)
        (:Is%20Valid
          (Variables|/Game/HelloUnreal/BP_MoveStair.BP_MoveStair_C|SetIsPlay (Variables|Default|GetMoveStair) true))
        (:Is%20Not%20Valid
          (Development|PrintString "MoveStair is Nullptr!!" true true "(R=0.520001,G=0.000000,B=0.000000,A=1.000000)"))))
    (:then_3
      (Utilities|IsValid (Variables|Default|GetSpawner)
        (:Is%20Valid
          (Default|DoSpawn (Variables|Default|GetSpawner)))
        (:Is%20Not%20Valid
          (Development|PrintString "Spawner is Nullptr!!" true true "(R=0.520001,G=0.000000,B=0.000000,A=1.000000)"))))))

(event OnComponentEndOverlap(Cube)
  (params (OverlappedComponent :type Primitive%20Component%20Object%20Reference) (OtherActor :type Actor%20Object%20Reference) (OtherComp :type Primitive%20Component%20Object%20Reference) (OtherBodyIndex :type Integer))
  (Development|PrintString (Utilities|String|Append "End Overlap" "Overlapped Component :" (Utilities|GetDisplayName OverlappedComponent) ". Other Actor :" (Utilities|GetDisplayName OtherActor) ". Other Comp :" (Utilities|GetDisplayName OtherComp)) true true "(R=0.000000,G=0.660000,B=1.000000,A=1.000000)" 6e+01)
  (Utilities|FlowControl|Sequence
    (:then_0
      (Utilities|IsValid (Variables|Default|GetMoveActor)
        (:Is%20Valid
          (Variables|/Game/HelloUnreal/BP_MoveActor.BP_MoveActor_C|SetIsPlay (Variables|Default|GetMoveActor) false))
        (:Is%20Not%20Valid
          (Development|PrintString "MoveActor is Nullptr!!" true true "(R=0.520001,G=0.000000,B=0.000000,A=1.000000)"))))
    (:then_1
      (Utilities|IsValid (Variables|Default|GetMoveRect)
        (:Is%20Valid
          (Variables|/Game/HelloUnreal/BP_MoveRect.BP_MoveRect_C|SetIsPlay (Variables|Default|GetMoveRect) false))
        (:Is%20Not%20Valid
          (Development|PrintString "MoveRect is Nullptr!!" true true "(R=0.520001,G=0.000000,B=0.000000,A=1.000000)"))))
    (:then_2
      (Utilities|IsValid (Variables|Default|GetMoveStair)
        (:Is%20Valid
          (Variables|/Game/HelloUnreal/BP_MoveStair.BP_MoveStair_C|SetIsPlay (Variables|Default|GetMoveStair) false))
        (:Is%20Not%20Valid
          (Development|PrintString "MoveStair is Nullptr!!" true true "(R=0.520001,G=0.000000,B=0.000000,A=1.000000)"))))))

(fn ConstructionScript)