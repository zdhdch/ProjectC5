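; BP_switch1 is a trigger switch that pauses three movers, MoveActor, MoveRect and MoveStair, while something overlaps its Cube component.
; Begin overlap sets IsPlay to false on all three references, and end overlap sets it back to true without filtering the other actor or counting overlaps.
; Both events also print the overlapped component, other actor and other component names to screen for debugging.
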(event OnComponentBeginOverlap(Cube)
  (params (OverlappedComponent :type Primitive%20Component%20Object%20Reference) (OtherActor :type Actor%20Object%20Reference) (OtherComp :type Primitive%20Component%20Object%20Reference) (OtherBodyIndex :type Integer) (bFromSweep :type Boolean) (SweepResult :type Hit%20Result%20Structure%20%28by%20ref%29))
  (Development|PrintString (Utilities|String|Append "Begin Overlap" "Overlapped Component :" (Utilities|GetDisplayName OverlappedComponent) ". Other Actor :" (Utilities|GetDisplayName OtherActor) ". Other Comp :" (Utilities|GetDisplayName OtherComp)) true true "(R=0.000000,G=0.660000,B=1.000000,A=1.000000)" 6e+01)
  (Variables|/Game/HelloUnreal/BP_MoveActor.BP_MoveActor_C|SetIsPlay (Variables|Default|GetMoveActor) false)
  (Variables|/Game/HelloUnreal/BP_MoveRect.BP_MoveRect_C|SetIsPlay (Variables|Default|GetMoveRect) false)
  (Variables|/Game/HelloUnreal/BP_MoveStair.BP_MoveStair_C|SetIsPlay (Variables|Default|GetMoveStair) false))

(event OnComponentEndOverlap(Cube)
  (params (OverlappedComponent :type Primitive%20Component%20Object%20Reference) (OtherActor :type Actor%20Object%20Reference) (OtherComp :type Primitive%20Component%20Object%20Reference) (OtherBodyIndex :type Integer))
  (Development|PrintString (Utilities|String|Append "End Overlap" "Overlapped Component :" (Utilities|GetDisplayName OverlappedComponent) ". Other Actor :" (Utilities|GetDisplayName OtherActor) ". Other Comp :" (Utilities|GetDisplayName OtherComp)) true true "(R=0.000000,G=0.660000,B=1.000000,A=1.000000)" 6e+01)
  (Variables|/Game/HelloUnreal/BP_MoveActor.BP_MoveActor_C|SetIsPlay (Variables|Default|GetMoveActor) true)
  (Variables|/Game/HelloUnreal/BP_MoveRect.BP_MoveRect_C|SetIsPlay (Variables|Default|GetMoveRect) true)
  (Variables|/Game/HelloUnreal/BP_MoveStair.BP_MoveStair_C|SetIsPlay (Variables|Default|GetMoveStair) true))

(fn ConstructionScript)