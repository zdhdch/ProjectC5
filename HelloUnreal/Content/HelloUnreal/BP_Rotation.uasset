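; BP_Rotation is an actor that rotates or oscillates a cube around an axis set by an Arrow component.
; At BeginPlay, if Play is set, it waits, moves Pivot to the Arrow's location and counter-offsets the Cube.
; A Timeline, optionally looping and rate-scaled by Duration, lerps Pivot's rotation around the Arrow's forward vector by the Oscillaton angle.
; Start and Stop events control the Timeline.
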(event Custom|Start
  (Components|Timeline|SetPlayRate (Variables|Default|GetTimeline) (/ 1.0 (Variables|Default|Getduration)))
  (bind _a (Timeline|Timeline Play)
    (:Update
      (Transformation|SetRelativeRotation (Variables|Default|GetPivot) (Math|Rotator|Lerp(Rotator) "0, 0, 0" (* (Math|Vector|RotatorfromAxisandAngle (Math|Vector|GetForwardVector (Variables|Default|GetArrow)) 1.0) (Variables|Default|Getoscillaton)) _a) false false))))

(event Custom|Stop
  (bind _a (Timeline|Timeline Stop)
    (:Update
      (Transformation|SetRelativeRotation (Variables|Default|GetPivot) (Math|Rotator|Lerp(Rotator) "0, 0, 0" (* (Math|Vector|RotatorfromAxisandAngle (Math|Vector|GetForwardVector (Variables|Default|GetArrow)) 1.0) (Variables|Default|Getoscillaton)) _a) false false))))

(event EventBeginPlay
  (if (Variables|Default|Getplay)
    (Utilities|FlowControl|Delay (Variables|Default|Gettime))
    (CallFunction|UpdatePivotLocation)
    (CallFunction|Start)))

(event Collision|EventActorBeginOverlap
  (params (OtherActor :type Actor%20Object%20Reference)))

(event EventTick
  (params (DeltaSeconds :type Float%20%28single-precision%29)))

(fn ConstructionScript
  (Components|Timeline|SetLooping (Variables|Default|GetTimeline) (Variables|Default|Getlooping)))

(fn UpdatePivotLocation
  (Transformation|SetRelativeLocation (Variables|Default|GetPivot) (Variables|/Script/Engine.SceneComponent|GetRelativeLocation (Variables|Default|GetArrow)) false false)
  (Transformation|SetRelativeLocation (Variables|Default|Getcube) (* (Variables|/Script/Engine.SceneComponent|GetRelativeLocation (Variables|Default|GetArrow)) -1.0) false false))